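; Survivor character that walks to given points by scripted interpolation, with standard character movement disabled on BeginPlay.
; PathFind flattens start and target to Z=0, turns the actor along the travel direction, then lerps its location on a timeline without sweeping.
; The timeline's play rate scales with WalkSpeed over distance, keeping travel speed independent of path length.
; ToggleMarker shows or hides the survivor's marker component.
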(event `self.ReceiveBeginPlay`
  (`CharacterMovementComponent.DisableMovement` (`self.CharacterMovement`)))

(event `PathFind`
  (params (TargetLocation :type "Vector Structure"))
  ;[0.02083 0.001995 0] LerpTo
  ;;[0 0 0] Establish XY locations
  (set `self.TargetLocation` (`KismetMathLibrary.MakeVector` (.x TargetLocation) (.y TargetLocation)))
  (set `self.LastLocation` (`KismetMathLibrary.MakeVector` (.x (`self.K2_GetActorLocation`)) (.y (`self.K2_GetActorLocation`))))
  ;;[0 0 0] Set Actor rotation
  (`self.K2_SetActorRotation` (`KismetMathLibrary.ComposeRotators` (`KismetMathLibrary.Conv_VectorToRotator` (`KismetMathLibrary.MakeVector` (.x (- (`self.LastLocation`) (`self.TargetLocation`))) (.y (- (`self.LastLocation`) (`self.TargetLocation`))))) (struct :`Yaw` 180.0)))
  ;;[0 0 0] LerpTo Location
  (`TimelineComponent.SetPlayRate` (`self.GotoTimeline`) (* (/ 1.0 (`KismetMathLibrary.MapRangeUnclamped` (`KismetMathLibrary.Vector_Distance` (`self.TargetLocation`) (`self.LastLocation`)) 0.0 100.0 0.0 1.0)) (`self.WalkSpeed`)))
  (bind (_direction _blend) (`Timeline|GotoTimeline` :!via `PlayFromStart`)
    (:`Update`
      (`self.K2_SetActorLocation` (`KismetMathLibrary.VLerp` (`self.LastLocation`) (`self.TargetLocation`) _blend)))))

(fn `ToggleMarker`
  (params (OnOff :type Boolean))
  (`SceneComponent.SetVisibility` (`self.Marker`) OnOff false))

(fn `UserConstructionScript`)