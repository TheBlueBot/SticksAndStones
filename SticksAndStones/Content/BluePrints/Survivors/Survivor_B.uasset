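; Survivor actor that walks to target locations and harvests resource nodes, with a widget showing its name, inventory and task progress.
; On BeginPlay it picks a random data-table name and fills the widget.
; PathFind moves it by straight timeline lerp at Z=0, scaling play rate by distance and WalkSpeed rather than using navigation.
; Arrival at a Resource-tagged target starts a timed harvest that blocks new moves, then calls the node's HarvestF.
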(event `self.ReceiveBeginPlay`
  (`self.RandName`)
  (`self.UpdateInv`))

(event `PathFind`
  (params (TargetLocation :type "Vector Structure") (TargetType :type "Actor Object Reference"))
  ;[0.02083 0.001995 0] LerpTo
  (set `self.Target` TargetType)
  (if (`self.CanMove`)
    ;;[0 0 0] Establish XY locations
    (set `self.TargetLocation` (`KismetMathLibrary.MakeVector` (.x TargetLocation) (.y TargetLocation)))
    (set `self.LastLocation` (`KismetMathLibrary.MakeVector` (.x (`self.K2_GetActorLocation`)) (.y (`self.K2_GetActorLocation`))))
    ;;[0 0 0] Set Actor rotation
    (`self.K2_SetActorRotation` (`KismetMathLibrary.ComposeRotators` (`KismetMathLibrary.Conv_VectorToRotator` (`KismetMathLibrary.MakeVector` (.x (- (`self.LastLocation`) (`self.TargetLocation`))) (.y (- (`self.LastLocation`) (`self.TargetLocation`))))) (struct :`Yaw` 180.0)))
    ;;[0 0 0] LerpTo Location
    (`TimelineComponent.SetPlayRate` (`self.Goto Timeline`) (* (/ 1.0 (`KismetMathLibrary.MapRangeUnclamped` (`KismetMathLibrary.Vector_Distance` (`self.TargetLocation`) (`self.LastLocation`)) 0.0 100.0 0.0 1.0)) (`self.WalkSpeed`)))
    (bind (_direction _blend) (`Timeline|Goto Timeline` :!via `PlayFromStart`)
      (:`Update`
        (`self.K2_SetActorLocation` (`KismetMathLibrary.VLerp` (`self.LastLocation`) (`self.TargetLocation`) _blend)))
      (:`Finished`
        (if (`KismetArrayLibrary.Array_Contains` (`Actor.Tags` (`self.Target`)) "Resource")
          (`self.Harvest Surv`))))))

(event `Harvest Surv`
  ;[0 0 0] Resource Harvest
  (bind _asresource_node (cast `/Game/BluePrints/Resources/Resource_Node` (`self.Target`)))
  (set `self.CanMove` false)
  (bind _assurvivor_ui (cast `/Game/BluePrints/UI/SurvivorUI` (`WidgetComponent.GetWidget` (`self.SurvivorHUD`))))
  (`TimelineComponent.SetPlayRate` (`self.LerpTime`) (/ 1.0 (`/Game/BluePrints/Resources/Resource_Node.HarvestRate` _asresource_node)))
  (bind (_direction _alpha) (`Timeline|LerpTime` :!via `PlayFromStart`)
    (:`Update`
      (set `/Game/BluePrints/UI/SurvivorUI.TaskCompletionUI` (`KismetMathLibrary.Lerp` 0.0 1.0 _alpha) _assurvivor_ui))
    (:`Finished`
      (set `self.CanMove` true)
      (`/Game/BluePrints/Resources/Resource_Node.Harvest_F` _asresource_node self))))

(fn `RandName`
  (bind _outrownames (`DataTableFunctionLibrary.GetDataTableRowNames` "/Game/BluePrints/Structs/RandomNames.RandomNames"))
  (bind _returnvalue (`|GetDataTableRow` "/Game/BluePrints/Structs/RandomNames.RandomNames" (`KismetStringLibrary.Conv_StringToName` (`KismetStringLibrary.Conv_IntToString` (`KismetMathLibrary.RandomInteger` (`KismetArrayLibrary.Array_Length` _outrownames)))))
    (:`then`
      (bind _firstname (break `/Game/BluePrints/Structs/StrName` _returnvalue))
      (`KismetSystemLibrary.PrintString` _firstname)
      (bind _output_get (set `self.Name` _firstname))
      (bind _assurvivor_ui (cast `/Game/BluePrints/UI/SurvivorUI` (`WidgetComponent.GetWidget` (`self.SurvivorHUD`))))
      (set `/Game/BluePrints/UI/SurvivorUI.SurvName` (`KismetTextLibrary.Conv_StringToText` _output_get) _assurvivor_ui))))

(fn `ToggleUI`
  (params (OnOff :type Boolean))
  (`SceneComponent.SetVisibility` (`self.SurvivorHUD`) OnOff false))

(fn `UpdateInv`
  (bind _assurvivor_ui (cast `/Game/BluePrints/UI/SurvivorUI` (`WidgetComponent.GetWidget` (`self.SurvivorHUD`))))
  (`/Game/BluePrints/UI/SurvivorUI.UpdateInventory` _assurvivor_ui (`self.Inventory`)))

(fn `UserConstructionScript`)