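; WorldGrid is an actor that procedurally generates a centered grid of tile actors on BeginPlay.
; A first pass samples FastNoise simplex fractal noise per cell, maps it to an AllTiles index, prints that index and appends the tile class to GridTiles.
; A second pass spawns those classes at 100-unit spacing, indexing GridTiles by the product of row and column rather than a row-major offset.
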(event `self.ReceiveBeginPlay`
  (bind _depth (`self.Depth`))
  (bind _width (`self.Width`))
  (`|ExecutionSequence`
    (:`then_0`
      ;[1 1 1] GenerateLayout
      (for _index (range (+ (`self.Width`) 1))
        (for _index_2 (range (+ (`self.Depth`) 1))
          (`self.ProcGen` _index_2 _index))))
    (:`then_1`
      ;[1 1 1] SpawnTiles
      (for _index_3 (range (+ _width 1))
        (for _index_4 (range (+ _depth 1))
          (`|SpawnActorFromClass` (`|GetArrayItem` (`self.Grid_Tiles`) (* _index_3 _index_4)) (`KismetMathLibrary.MakeTransform` (`KismetMathLibrary.MakeVector` (`KismetMathLibrary.Conv_IntToDouble` (* (- _index_4 (/ _depth 2)) 100)) (`KismetMathLibrary.Conv_IntToDouble` (* (- _index_3 (/ _width 2)) 100)))) "Undefined" "OverrideRootScale" null null))))))

(fn `ProcGen`
  (params (X :type Integer) (Y :type Integer))
  (returns (Output :type "Actor Class Reference") (ObjectList :type "Array of Actor Class Reference"))
  (bind _alltiles (`self.AllTiles`))
  (bind _returnvalue (`self.FastNoise`))
  (bind _returnvalue_2 (`KismetMathLibrary.Round` (`KismetMathLibrary.MapRangeClamped` (`FastNoiseWrapper.GetNoise2D` _returnvalue (* (`KismetMathLibrary.Conv_IntToDouble` X) 20.0) (* (`KismetMathLibrary.Conv_IntToDouble` Y) 20.0)) -1.0 1.0 0.0 (`KismetMathLibrary.Conv_IntToDouble` (- (`KismetArrayLibrary.Array_Length` _alltiles) 1)))))
  (`KismetSystemLibrary.PrintText` (`KismetTextLibrary.Conv_IntToText` _returnvalue_2) true true (struct :`G` 0.66 :`B` 1.0 :`A` 1.0) 12.0)
  ;[1 1 1] Add Tile to grid
  (`KismetArrayLibrary.Array_Add` (`self.Grid_Tiles`) (`|GetArrayItem` _alltiles _returnvalue_2))
  (return null))

(fn `UserConstructionScript`)