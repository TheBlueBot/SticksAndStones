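; Player controller Blueprint for click-based selection and movement of Survivor_BP units.
; On left click, a cursor trace stores any survivor hit as SelectedSurvivor, or sends the selected survivor's PathFind to a clicked "Tile" actor's location.
; Each click also updates every survivor's marker so only the selected one is flagged.
; SetHighlight is an unused, unfinished outline helper that only prints debug text, with its mesh and material nodes disconnected.
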(event `InputAction|LeftClick`
  (params (Key :type "Key Structure"))
  (bind (_bblockinghit _binitialoverlap _time _distance _location _impactpoint _normal _impactnormal _physmat _hitactor) (`GameplayStatics.BreakHitResult` (`self.GetHitResultUnderCursorByChannel` "TraceTypeQuery1")))
  (bind _returnvalue (`self.K2_GetActorLocation` _hitactor))
  (:`Pressed`
    (`|ExecutionSequence`
      (:`then_0`
        ;[0 0 0] Set last selected survivor
        (cast `/Game/BluePrints/Survivors/Survivor_BP` _hitactor)
        (set `self.SelectedSurvivor` _hitactor))
      (:`then_1`
        ;[0 0 0] Function Pathfind where clicked
        (if (`KismetArrayLibrary.Array_Contains` (`Actor.Tags` _hitactor) "Tile")
          (bind _assurvivor_bp (cast `/Game/BluePrints/Survivors/Survivor_BP` (`self.SelectedSurvivor`)))
          (`/Game/BluePrints/Survivors/Survivor_BP.PathFind` _assurvivor_bp _returnvalue)
          (`KismetSystemLibrary.PrintString` (`KismetStringLibrary.Conv_VectorToString` _returnvalue) true true (struct :`G` 0.66 :`B` 1.0 :`A` 1.0) 5.0)))
      (:`then_2`
        ;[0 0 0] Comment
        (bind _outactors (`GameplayStatics.GetAllActorsOfClass` "/Game/BluePrints/Survivors/Survivor_BP.Survivor_BP_C"))
        (for _array_element _outactors
          (bind _assurvivor_bp_2 (cast `/Game/BluePrints/Survivors/Survivor_BP` _array_element))
          (`/Game/BluePrints/Survivors/Survivor_BP.ToggleMarker` _assurvivor_bp_2 (== _array_element (`self.SelectedSurvivor`))))))))

(fn `SetHighlight`
  (params (InputPin :type "Actor Object Reference"))
  ;[0 0 0] SetHighlight
  (if (== (`GameplayStatics.GetObjectClass` InputPin) "/Game/BluePrints/Survivors/Survivor_BP.Survivor_BP_C")
    (for _index (range (`KismetArrayLibrary.Array_Length` (`self.K2_GetComponentsByClass` InputPin "/Script/Engine.StaticMeshComponent")))
      (`KismetSystemLibrary.PrintString` "Hello"))))

(fn `UserConstructionScript`)