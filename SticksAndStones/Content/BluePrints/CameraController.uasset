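; Player-driven camera rig that pans across the level and zooms, and opens the objectives UI.
; Each Tick moves the root along normalized input axes, scaling speed up with zoom distance, and slides the Camera along local X within clamped zoom limits.
; The construction script aims CameraHold at the Focus component.
; BeginPlay adds a child actor component; each Tab press creates and focuses a new ObjectivesQueue widget, with no hide logic.
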(event `self.ReceiveBeginPlay`
  (`AddComponent|NODE_AddChildActorComponent-1`))

(event `self.ReceiveTick`
  (params (DeltaSeconds :type "Float (single-precision)"))
  (`SceneComponent.K2_AddRelativeLocation` (`self.DefaultSceneRoot`) (* (`KismetMathLibrary.Normal` (`KismetMathLibrary.MakeVector` (`self.GetInputAxisValue`) (`self.GetInputAxisValue`))) (* (`self.MovementSpeed`) (+ (/ (* (`self.Zoom_f`) -1.0) 1000.0) 1.0))) false false)
  ;[0 0 0] Recieve Zoom input, Clamp, then apply
  (set `self.Zoom_f` (`KismetMathLibrary.FClamp` (+ (`self.Zoom_f`) (* (`self.GetInputAxisValue`) 300.0)) -8000.0 -200.0))
  (`SceneComponent.K2_SetRelativeLocation` (`self.Camera`) (`KismetMathLibrary.MakeVector` (`self.Zoom_f`)) false false))

(event `Key|Tab`
  (params (Key :type "Key Structure"))
  ;[0 0 0] Show/Hide Objective UI
  (:`Pressed`
    (bind _returnvalue (`|CreateWidget` "/Game/BluePrints/UI/ObjectivesQueue.ObjectivesQueue_C" (`GameplayStatics.GetPlayerController` 0)))
    (`UserWidget.AddToViewport` _returnvalue 0)
    (`Widget.SetFocus` _returnvalue)))

(fn `UserConstructionScript`
  (bind _camerahold (`self.CameraHold`))
  ;[0 0 0] Point Camera at origin
  (`SceneComponent.K2_SetRelativeRotation` _camerahold (`KismetMathLibrary.FindLookAtRotation` (`SceneComponent.K2_GetComponentLocation` _camerahold) (`SceneComponent.K2_GetComponentLocation` (`self.Focus`))) false false))